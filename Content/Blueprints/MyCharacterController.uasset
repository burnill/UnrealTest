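; Player-controlled tornado character that destroys whatever it hits and grows larger with each hit.
; Axis inputs drive camera pitch, forward movement along control rotation, and yaw steering, with dampener variables dividing the move and turn rates.
; Tick spins the Cone mesh at a fixed per-frame rate, while Hit destroys the other actor without filtering and adds ScaleAmount to actor scale.
; Strafing is unused, and the boost and normal speed functions are empty stubs.
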(event EventTick
  (params (DeltaSeconds :type Float%20%28single-precision%29))
  ;[1 1 1] Rotate Tornado Mesh
  (Transformation|AddWorldRotation (Variables|Default|GetCone) "0.000000,3.500000,0.000000" false false))

(event Collision|EventHit
  (params (MyComp :type Primitive%20Component%20Object%20Reference) (Other :type Actor%20Object%20Reference) (OtherComp :type Primitive%20Component%20Object%20Reference) (bSelfMoved :type Boolean) (HitLocation :type Vector :default "0, 0, 0") (HitNormal :type Vector :default "0, 0, 0") (NormalImpulse :type Vector :default "0, 0, 0") (Hit :type Hit%20Result%20Structure%20%28by%20ref%29))
  (bind _returnvalue (Transformation|GetActorScale3D))
  (bind _scaleamount (Variables|Default|GetScaleAmount))
  (bind (_x _y _z) (Math|Vector|BreakVector _returnvalue))
  ;[1 1 1] BuildingCollision
  (Actor|DestroyActor Other)
  (Transformation|SetActorScale3D (Math|Vector|MakeVector (+ _x _scaleamount) (+ _y _scaleamount) (+ _z _scaleamount))))

(event Input|AxisEvents|InputAxisForward_Backward
  (params (AxisValue :type Float%20%28single-precision%29))
  ;[1 1 1] U, D, L, R
  (Pawn|Input|AddMovementInput (Math|Vector|GetForwardVector (Pawn|GetControlRotation :!class /Script/Engine.Pawn)) (/ AxisValue (Variables|Default|GetMoveSpeedDampner)) false))

(event Input|AxisEvents|InputAxisLeft_Right
  (params (AxisValue :type Float%20%28single-precision%29))
  ;[1 1 1] Rotate Camera
  (Pawn|Input|AddControllerYawInput (/ AxisValue (Variables|Default|GetRotationSpeedDampner))))

(event Input|AxisEvents|InputAxisLooking_Up_Down
  (params (AxisValue :type Float%20%28single-precision%29))
  ;[1 1 1] Rotate Camera
  (Pawn|Input|AddControllerPitchInput AxisValue))

(fn ConstructionScript)

(fn AddActorLocalRotation
  (params (Delta%20Rotation :type Rotator)))

(fn BoostSpeed
  (params (BoostSpeedIn :type Float%20%28single-precision%29))
  (return 0.0))

(fn NormalSpeed
  (params (NormalSpeedIn :type Float%20%28single-precision%29))
  (return 0.0))